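; BP_WeatherController is a weather actor that runs a scripted rain cycle at level start.
; BeginPlay hands rain sound and particles to RainComponent, then uses delays to shift cloud and gloom targets and toggle rain on, then off.
; The particle system snaps to the player camera manager to follow the view.
; Each tick, CloudComponent updates SkySphere cloud opacity, using the rain change rate and a global material parameter instance.
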(event EventBeginPlay
  (bind _cloudcomponent (Variables|Default|GetCloudComponent))
  (bind _cloudcomponent_2 (Variables|Default|GetCloudComponent))
  (Utilities|Init)
  (Utilities|FlowControl|Delay 0.2)
  (Variables|/Script/OpenWorld.CloudComponent|SetTargetCloudOpacity _cloudcomponent_2 8.0)
  (Variables|/Script/OpenWorld.CloudComponent|SetTargetGloomLevel _cloudcomponent_2 0.1)
  (Utilities|FlowControl|Delay 5.0)
  (Class|WeatherController|OnToggleRain true)
  (Utilities|FlowControl|Delay 3e+01)
  (Class|WeatherController|OnToggleRain false)
  (Variables|/Script/OpenWorld.CloudComponent|SetTargetCloudOpacity _cloudcomponent 0.7)
  (Variables|/Script/OpenWorld.CloudComponent|SetTargetGloomLevel _cloudcomponent 1.0))

(event Collision|EventActorBeginOverlap
  (params (OtherActor :type Actor%20Object%20Reference)))

(event EventTick
  (params (DeltaSeconds :type Float%20%28single-precision%29))
  (Utilities|UpdateSky))

(fn ConstructionScript)